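; Item spawner actor that keeps an item of ItemClass at each of its four spawn locations.
; BeginPlay spawns one item per location and stores them in SpawnedItem, in the same order as the locations.
; Tick runs through a four-second Delay, then spawns a replacement at the matching location for any hidden item and overwrites its array slot.
; Hidden items are not destroyed here.
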(event EventBeginPlay
  (bind _output_get (Variables|Default|SetLocArray (Utilities|Array|MakeArray (Variables|Default|GetSpawnLoc1) (Variables|Default|GetSpawnLoc2) (Variables|Default|GetSpawnLoc3) (Variables|Default|GetSpawnLoc4))))
  (for _array_element _output_get
    (bind _returnvalue (Game|SpawnActorfromClass (Variables|Default|GetItemClass) (Transformation|GetWorldTransform _array_element) "Undefined" 0 0))
    (Utilities|Array|Add (Variables|Default|GetSpawnedItem) _returnvalue)))

(event EventTick
  (params (DeltaSeconds :type Float%20%28single-precision%29))
  (Utilities|FlowControl|Delay 4.0)
  (for (_array_element _array_index) (Variables|Default|GetSpawnedItem)
    (if (Variables|/Script/Engine.Actor|GetbHidden _array_element)
      (bind _returnvalue (Game|SpawnActorfromClass (Variables|Default|GetItemClass) (Transformation|GetWorldTransform (Utilities|Array|Get(acopy) (Variables|Default|GetLocArray) _array_index)) "Undefined" 0 0))
      (Utilities|Array|SetArrayElem (Variables|Default|GetSpawnedItem) _array_index _returnvalue))))

(fn ConstructionScript)